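; Shared two-player camera actor that becomes player controller 0's view target on BeginPlay and keeps following both players.
; Each tick it eases the spring arm length toward the players' horizontal separation, clamped to a minimum, and eases itself toward their midpoint at Z zero.
; Both updates share one interpolation speed and read the players from the InputHandler actor, looked up by class on each call.
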(event EventBeginPlay
  (Game|Player|SetViewTargetwithBlend (Game|GetPlayerController 0) self 0.0 "VTBlend_Linear" 0.0 false))

(event Collision|EventActorBeginOverlap
  (params (OtherActor :type Actor%20Object%20Reference)))

(event EventTick
  (params (DeltaSeconds :type Float%20%28single-precision%29))
  (CallFunction|UpdateArmLength DeltaSeconds)
  (CallFunction|UpdateLocation DeltaSeconds))

(fn ConstructionScript)

(fn UpdateArmLength
  (params (DeltaTime :type Float%20%28single-precision%29))
  (bind (_player0 _player1) (CallFunction|GetPlayers))
  (bind _output_get (Variables|Default|SetPreviousArmLength (Math|Interpolation|FInterpTo (Variables|Default|GetPreviousArmLength) (Math|Float|Max(Float) (Math|Vector|Distance(Vector) (Math|Vector|MakeVector (.X (Math|Vector|BreakVector (Transformation|GetActorLocation _player0))) (.Y (Math|Vector|BreakVector (Transformation|GetActorLocation _player0))) 0.0) (Math|Vector|MakeVector (.X (Math|Vector|BreakVector (Transformation|GetActorLocation _player1))) (.Y (Math|Vector|BreakVector (Transformation|GetActorLocation _player1))) 0.0)) (Variables|Default|GetMinSideArmLenth)) DeltaTime (Variables|Default|GetInterpolationSpeed))))
  (Variables|/Script/Engine.SpringArmComponent|SetTargetArmLength (Variables|Default|GetSpringArm) _output_get))

(fn UpdateLocation
  (params (DeltaTime :type Float%20%28single-precision%29))
  (bind (_player0 _player1) (CallFunction|GetPlayers))
  (bind _output_get (Variables|Default|SetPreviousLocation (Math|Interpolation|VInterpTo (Variables|Default|GetPreviousLocation) (/ (+ (Math|Vector|MakeVector (.X (Math|Vector|BreakVector (Transformation|GetActorLocation _player0))) (.Y (Math|Vector|BreakVector (Transformation|GetActorLocation _player0))) 0.0) (Math|Vector|MakeVector (.X (Math|Vector|BreakVector (Transformation|GetActorLocation _player1))) (.Y (Math|Vector|BreakVector (Transformation|GetActorLocation _player1))) 0.0)) 2.0) DeltaTime (Variables|Default|GetInterpolationSpeed))))
  (Transformation|SetActorLocation _output_get false false))

(fn GetPlayers
  (bind _returnvalue (Actor|GetActorOfClass "/Script/GGJ2020.InputHandler"))
  (return (Variables|/Script/GGJ2020.InputHandler|Getm_Player1 _returnvalue) (Variables|/Script/GGJ2020.InputHandler|Getm_Player2 _returnvalue)))