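; BP_ResourcePickable is a pickable actor that carries a resource essence.
; On BeginPlay it runs the parent logic, spawns a ResourceEssence actor at its own location and stores it in PickableEssence.
; The Blueprint adds no other behavior: its overlap and tick events are disabled stubs, and its construction script only calls the parent.
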(event EventBeginPlay
  (|CallParentFunction)
  (bind _returnvalue (Game|SpawnActorfromClass "/Script/GGJ2020.ResourceEssence" (Math|Conversions|ToTransform(Vector) (Transformation|GetActorLocation)) "Undefined" 0 0))
  (Variables|Default|SetPickableEssence _returnvalue))

(event Collision|EventActorBeginOverlap
  (params (OtherActor :type Actor%20Object%20Reference))
  (|CallParentFunction OtherActor) ; This node is disabled and will not be called.\nDrag off pins to build functionality.
)

(event EventTick
  (params (DeltaSeconds :type Float%20%28single-precision%29))
  (|CallParentFunction DeltaSeconds) ; This node is disabled and will not be called.\nDrag off pins to build functionality.
)

(fn ConstructionScript
  (|CallParentFunction))