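; Projectile Blueprint that flies along a set direction and destroys itself once it passes its maximum range from where it spawned.
; BeginPlay records the mesh's start position, and Tick compares squared distance from it against the range limit, printing that value for debugging.
; Movement is a fixed step per frame without sweep or delta-time scaling.
; The overlap event is empty, so no hit handling exists here.
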(event EventBeginPlay
  (Variables|Default|SetStartPosition (Transformation|GetWorldLocation (Variables|Default|GetMeshBody))))

(event Collision|EventActorBeginOverlap
  (params (OtherActor :type Actor%20Object%20Reference)))

(event EventTick
  (params (DeltaSeconds :type Float%20%28single-precision%29))
  (bind _startposition (Variables|Default|GetStartPosition))
  (bind _meshbody (Variables|Default|GetMeshBody))
  (bind _returnvalue (Transformation|GetWorldLocation _meshbody))
  (bind _returnvalue_2 (- _returnvalue _startposition))
  (bind _returnvalue_3 (Math|Vector|VectorLengthSquared _returnvalue_2))
  (if (< _returnvalue_3 (* 2.5e+04 2.5e+04))
    (Development|PrintString (Utilities|String|ToString(Float) _returnvalue_3))
    (Transformation|SetWorldLocation _meshbody (+ _returnvalue (* (Variables|Default|GetmoveDirection) 25.0)) false false)
    (else
      (Actor|DestroyActor))))

(fn ConstructionScript)