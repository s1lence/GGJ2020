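; TilesManager_BP is a manager Blueprint that builds and keeps track of a 30 by 30 grid of Tile actors.
; The Construction Script adds each tile as a Child Actor Component, using modulo and division on the loop index to place it at 100-unit spacing.
; Each spawned child is cast to Tile and appended to the MTiles array.
; The Event Graph holds only disabled default events, so it adds no runtime logic.
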(event EventBeginPlay)

(event Collision|EventActorBeginOverlap
  (params (OtherActor :type Actor%20Object%20Reference)))

(event EventTick
  (params (DeltaSeconds :type Float%20%28single-precision%29)))

(fn ConstructionScript
  (for _index (range 0 899)
    (bind _returnvalue (AddComponent|AddChildActorComponent false))
    (ChildActorComponent|SetChildActorClass _returnvalue "/Script/GGJ2020.Tile")
    (Transformation|SetRelativeLocation _returnvalue (Math|Vector|MakeVector (* (Math|Integer|%(Integer) _index 30) 1e+02) (* (/ _index 30) 1e+02) 0.0) false false)
    (bind _astile (Utilities|Casting|CastToTile (Variables|/Script/Engine.ChildActorComponent|GetChildActor _returnvalue)))
    (Utilities|Array|Add (Variables|Default|Getm_Tiles) _astile)))